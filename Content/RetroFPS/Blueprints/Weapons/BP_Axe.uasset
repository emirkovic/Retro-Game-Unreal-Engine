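; BP_Axe is the axe weapon for a retro FPS, a child Blueprint that drives the weapon's flipbook sprite.
; Initializing the weapon shows the idle flipbook, and attacking plays the attack flipbook for its length before returning to idle.
; A timed point light flash event is defined but left unused, and the graph itself contains no hit or damage logic.
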(event `self.Initialize Weapon`
  ;[0 0 0] Equip Weapon
  (`PaperFlipbookComponent.SetFlipbook` (`self.Weapon Flipbook`) (`self.Idle Axe`))
  (`SceneComponent.SetHiddenInGame` (`self.Weapon Flipbook`) false false))

(event `Attack`
  (bind _weapon_flipbook (`self.Weapon Flipbook`))
  ;[0 0 0] Axe Attack Animation
  (`PaperFlipbookComponent.SetFlipbook` _weapon_flipbook (`self.Fire Axe`))
  (`KismetSystemLibrary.Delay` (`PaperFlipbookComponent.GetFlipbookLength` _weapon_flipbook))
  (`PaperFlipbookComponent.SetFlipbook` (`self.Weapon Flipbook`) (`self.Idle Axe`)))

(event `Light Flash`
  (bind _pointlight (`self.PointLight`))
  ;[0 0 0] Light Flash
  (`SceneComponent.SetHiddenInGame` _pointlight false false)
  (`KismetSystemLibrary.Delay` 0.25)
  (`SceneComponent.SetHiddenInGame` _pointlight true false))

(fn `UserConstructionScript`
  (`parent.UserConstructionScript`))
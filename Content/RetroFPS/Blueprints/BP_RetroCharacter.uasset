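; BP_RetroCharacter is a RetroFPS character Blueprint that handles damage, the death check and the pause menu.
; TakeDamage receives cue data, prints health and armor from the Ability System Component, and reports an AI damage-sense event using the effect context's instigator.
; HealthCheck then tests an attribute against zero and calls KillCharacter, an empty event here.
; PauseGame input toggles the pause widget and the game's paused state.
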(event `Take Damage`
  (params (`Cue Data` :type "GameplayCueParameters Structure"))
  (bind (_normalizedmagnitude _rawmagnitude _effectcontext _matchedtagname _originaltag _aggregatedsourcetags _aggregatedtargettags _location) (`AbilitySystemBlueprintLibrary.BreakGameplayCueParameters` `Cue Data`))
  (bind _abilitysystemcomponent (`self.AbilitySystemComponent`))
  (`KismetSystemLibrary.PrintString` (`KismetStringLibrary.Concat_StrStr` "Health: " (`KismetStringLibrary.Conv_DoubleToString` (`.ReturnValue` (`AbilitySystemBlueprintLibrary.GetFloatAttributeFromAbilitySystemComponent` _abilitysystemcomponent (struct :`AttributeName` "Health" :`Attribute` "/Script/Test.RetroFPSAttributeSet:Health" :`AttributeOwner` "/Script/CoreUObject.Class'/Script/Test.RetroFPSAttributeSet'")))) ".Armor: " (`KismetStringLibrary.Conv_DoubleToString` (`.ReturnValue` (`AbilitySystemBlueprintLibrary.GetFloatAttributeFromAbilitySystemComponent` _abilitysystemcomponent (struct :`AttributeName` "Armor" :`Attribute` "/Script/Test.RetroFPSAttributeSet:Armor" :`AttributeOwner` "/Script/CoreUObject.Class'/Script/Test.RetroFPSAttributeSet'"))))) true true (struct :`G` 0.66 :`B` 1.0 :`A` 1.0) 60.0)
  (`AISense_Damage.ReportDamageEvent` self (`AbilitySystemBlueprintLibrary.EffectContextGetInstigatorActor` _effectcontext) 0.0 _location)
  (if (`self.Health Check`)
    (`self.Kill Character`)))

(event `Kill Character`)

(event `EnhancedInput|/Game/RetroFPS/Input/Actions/PauseGame`
  (params (ActionValue :type Boolean) (ElapsedSeconds :type "Float (double-precision)") (TriggeredSeconds :type "Float (double-precision)") (InputAction :type "InputAction Object Reference" :default "/Game/RetroFPS/Input/Actions/PauseGame.PauseGame"))
  (:`Started`
    (if (not (`self.isPauseMenuOpen`))
      (set `self.isPauseMenuOpen` true)
      (bind _returnvalue (`|CreateWidget` "/Game/RetroFPS/UI/Pausemenu.Pausemenu_C" (`GameplayStatics.GetPlayerController` 0)))
      (bind _output_get (set `self.PauseMenuWidget` _returnvalue))
      (`UserWidget.AddToViewport` _output_get 0)
      (`GameplayStatics.SetGamePaused` true)
      (else
        (set `self.isPauseMenuOpen` false)
        (`Widget.RemoveFromParent` (`self.PauseMenuWidget`))
        (`GameplayStatics.SetGamePaused` false)))))

(fn `Health Check`
  (returns (`Is Dead?` :type Boolean))
  (return (<= (`.ReturnValue` (`AbilitySystemBlueprintLibrary.GetFloatAttributeFromAbilitySystemComponent` (`self.AbilitySystemComponent`) (struct :`AttributeName` "Health" :`Attribute` "/Script/Test.RetroFPSAttributeSet:Health" :`AttributeOwner` "/Script/CoreUObject.Class'/Script/Test.RetroFPSAttributeSet'"))) 0.0)))

(fn `UserConstructionScript`)
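; Retro FPS enemy character that runs a behavior tree and renders as a billboarded Paper2D flipbook with Doom-style eight-direction sprites.
; Each tick it yaws the sprite toward the camera, then uses dot products against the player direction and its velocity to pick a directional walk or idle flipbook.
; Damage briefly overrides this; death stops AI and collision, plays dying then dead flipbooks, and calls its spawner.
; Melee and ranged attack events are empty here.
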(event `self.ReceiveBeginPlay`
  (bind _asbp_retro_fpsenemy_ai (cast `/Game/RetroFPS/Blueprints/Enemies/AI/BP_RetroFPSEnemyAI` (`self.GetController`)))
  (`AIController.RunBehaviorTree` _asbp_retro_fpsenemy_ai (`self.Behavior Tree`)))

(event `self.ReceiveTick`
  (params (DeltaSeconds :type "Float (single-precision)"))
  (`self.Sprite Face Player`
    (:`Out`
      (if (not (or (`self.Is Dead`) (`self.Pause Angle Calculations`)))
        (`self.Get Enemy Angle`
          (:`Out`
            (`self.Check If Walking`
              (:`Out`
                (`self.Calculate Flipbook`)))))))))

(event `self.Kill Character`
  (bind _enemy (`self.Enemy`))
  (`parent.Kill Character`)
  (bind _asbp_retro_fpsenemy_ai (cast `/Game/RetroFPS/Blueprints/Enemies/AI/BP_RetroFPSEnemyAI` (`self.GetController`)))
  (`BrainComponent.StopLogic` (`AIController.BrainComponent` _asbp_retro_fpsenemy_ai) "")
  (set `self.Is Dead` true)
  (`PrimitiveComponent.SetCollisionEnabled` (`self.CapsuleComponent`) "NoCollision")
  (`PaperFlipbookComponent.SetFlipbook` _enemy (`self.Dying`))
  (`KismetSystemLibrary.Delay` (`PaperFlipbookComponent.GetFlipbookLength` _enemy))
  (`PaperFlipbookComponent.SetFlipbook` (`self.Enemy`) (`self.Dead`))
  (`/Game/RetroFPS/Blueprints/BP_EnemySpawner.Spawn Enemy` (`self.Spawner`)))

(event `self.Take Damage`
  (params (`Cue Data` :type "GameplayCueParameters Structure"))
  (bind _enemy (`self.Enemy`))
  (`parent.Take Damage` `Cue Data`)
  (if (not (`self.Is Dead`))
    (set `self.Pause Angle Calculations` true)
    (`PaperFlipbookComponent.SetFlipbook` _enemy (`self.Damaged`))
    (`KismetSystemLibrary.Delay` (`PaperFlipbookComponent.GetFlipbookLength` _enemy))
    (set `self.Pause Angle Calculations` false)))

(event `Melee Attack`)

(event `Ranged Attack`)

(fn `Set Flipbook`
  (params (Walking :type "PaperFlipbook Object Reference") (Idle :type "PaperFlipbook Object Reference"))
  (bind _enemy (`self.Enemy`))
  (if (`self.Is Walking`)
    (`PaperFlipbookComponent.SetFlipbook` _enemy Walking)
    (else
      (`PaperFlipbookComponent.SetFlipbook` _enemy Idle))))

(fn `UserConstructionScript`)
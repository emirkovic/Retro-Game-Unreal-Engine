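; BP_AxeEnemy is an axe enemy for a retro FPS, drawn as a billboarded flipbook sprite with eight-directional animation.
; Each Tick yaws the sprite toward the camera and, unless dead or paused, computes the player's angle to the enemy's facing using dot products.
; That angle, the visible side and movement velocity select a directional walking or idle flipbook.
; Attack briefly pauses this selection to show the Shooting flipbook, then signals attack end.
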(event `self.ReceiveBeginPlay`)

(event `self.ReceiveTick`
  (params (DeltaSeconds :type "Float (single-precision)"))
  (`self.Sprite Face Player`
    (:`Out`
      (if (not (or (`self.Is Dead`) (`self.Pause Angle Calculations`)))
        (`self.Get Enemy Angle`
          (:`Out`
            (`self.Check If Walking`
              (:`Out`
                (`self.Calculate Flipbook`)))))))))

(event `Attack`
  (set `self.Pause Angle Calculations` true)
  (`PaperFlipbookComponent.SetFlipbook` (`self.Enemy`) (`self.Shooting`))
  (`KismetSystemLibrary.Delay` 0.4)
  (set `self.Pause Angle Calculations` false)
  (`self.OnAttackEnd`))

(fn `Set Flipbook`
  (params (Walking :type "PaperFlipbook Object Reference") (Idle :type "PaperFlipbook Object Reference"))
  (bind _enemy (`self.Enemy`))
  (if (`self.Is Walking`)
    (`PaperFlipbookComponent.SetFlipbook` _enemy Walking)
    (else
      (`PaperFlipbookComponent.SetFlipbook` _enemy Idle))))

(fn `UserConstructionScript`)
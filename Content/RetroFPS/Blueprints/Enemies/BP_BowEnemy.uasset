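; BP_BowEnemy is a ranged enemy Blueprint for a retro FPS, drawn with flipbook sprites.
; Its RangedAttack event pauses angle calculations, switches to the Shooting flipbook and activates a Gameplay Ability by tag.
; Angle calculations resume after a short fixed delay, independent of the ability's completion.
; An unused, disconnected point light flash remains in the graph, and construction only calls the parent.
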(event `self.Ranged Attack`
  (set `self.Pause Angle Calculations` true)
  (`PaperFlipbookComponent.SetFlipbook` (`self.Enemy`) (`self.Shooting`))
  (`AbilitySystemComponent.TryActivateAbilitiesByTag` (`self.AbilitySystemComponent`) (`self.Gameplay Tag Container`) false)
  (`KismetSystemLibrary.Delay` 0.4)
  (set `self.Pause Angle Calculations` false))

(fn `UserConstructionScript`
  (`parent.UserConstructionScript`))
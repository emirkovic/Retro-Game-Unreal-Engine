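; Base Gameplay Ability for RetroFPS bullet weapons, with empty FireWeapon and Reset hooks.
; Activation commits, starts a gameplay event listener, calls FireWeapon, then ends after the remaining cooldown, so cooldown sets fire rate.
; ApplyEffect sends the weapon event tag with target data to the attacker, and the listener applies the GameplayEffect to that target.
; Ability end stops both async tasks, calling Reset if the delay task is valid.
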(event `self.K2_ActivateAbility`
  ;[0 0 0] Activation
  (`self.K2_CommitAbility`)
  (`self.Wait for Event`)
  (`self.Fire Weapon`)
  ;[0 0 0] Ability Duration
  (bind _asynctaskproxy (`GameplayTask_WaitDelay.TaskWaitDelay` null (`self.GetCooldownTimeRemaining`))
    (:`then`
      (set `self.Fire Rate Delay Task` _asynctaskproxy))
    (:`OnFinish`
      (`self.K2_EndAbility`))))

(event `Wait for Event`
  ;[0 0 0] Wait For Gameplay Tag
  (bind (_asynctaskproxy _payload) (`AbilityTask_WaitGameplayEvent.WaitGameplayEvent` (`self.Weapon Event Tag`) null)
    (:`then`
      (set `self.Gamepay Event Wait Task` _asynctaskproxy))
    (:`EventReceived`
      (`self.BP_ApplyGameplayEffectToTarget` (`.TargetData` (break `GameplayEventData` _payload)) (`self.Gameplay Effect`)))))

(event `Fire Weapon`
  ;[1 0.07087 0.8099] Override
)

(event `self.K2_OnEndAbility`
  (params (bWasCancelled :type Boolean))
  (bind _gamepay_event_wait_task (`self.Gamepay Event Wait Task`))
  (bind _fire_rate_delay_task (`self.Fire Rate Delay Task`))
  ;[0 0 0] End Ability Cleanup
  (`/Engine/EditorBlueprintResources/StandardMacros.IsValid` _gamepay_event_wait_task
    (:`Is Valid`
      (`GameplayTask.EndTask` _gamepay_event_wait_task))
    (:`Is Not Valid`
      _))
  (`/Engine/EditorBlueprintResources/StandardMacros.IsValid` _fire_rate_delay_task
    (:`Is Valid`
      (`GameplayTask.EndTask` _fire_rate_delay_task)
      (`self.Reset`))))

(fn `Apply Effect`
  (params (`Attacking Actor` :type "Actor Object Reference") (`Target Actor` :type "Actor Object Reference"))
  (`AbilitySystemBlueprintLibrary.SendGameplayEventToActor` `Attacking Actor` (`self.Weapon Event Tag`) (make `GameplayEventData` (struct) null `Target Actor` null null (struct) (struct) (struct) 0.0 (`AbilitySystemBlueprintLibrary.AbilityTargetDataFromActor` `Target Actor`))))

(fn `Reset`)
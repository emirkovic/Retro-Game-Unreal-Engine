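; BP_FPSPlayer is the retro FPS player character, handling movement, mouse look, weapon pickup and switching, firing, and HUD feedback.
; Weapons are looked up in DT_RetroFPSWeapons, stored in an owned array, and spawned through a child actor component that bobs during movement.
; Equipping sets a gameplay tag, which fire input uses to activate Gameplay Ability System abilities.
; Damage and item pickups refresh health and armor text and play timeline-driven screen flashes.
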(event `self.ReceiveBeginPlay`
  ;[0 0 0] Initialization
  (`parent.ReceiveBeginPlay`)
  (bind _returnvalue (`|CreateWidget` "/Game/RetroFPS/Blueprints/Widgets/WBP_HUD.WBP_HUD_C"))
  (bind _output_get (set `self.HUD` _returnvalue))
  (`UserWidget.AddToViewport` _output_get 0)
  (`KismetSystemLibrary.Delay` 0.0)
  (`self.Update UI`)
  (`self.Initialize Weapon` "/Game/RetroFPS/Blueprints/Player/BP_PlayerWeaponBase.BP_PlayerWeaponBase_C")
  (`/Game/RetroFPS/Blueprints/Widgets/WBP_HUD.Switch Weapon` (`self.HUD`) "NewEnumerator0"))

(event `InputAxis|HorizontalMovement`
  (params (AxisValue :type "Float (single-precision)"))
  (bind (_returnvalue_roll _returnvalue_pitch _returnvalue_yaw) (`KismetMathLibrary.BreakRotator` (`self.GetControlRotation`)))
  ;[0 0 0] Movement
  (`self.AddMovementInput` (`KismetMathLibrary.GetRightVector` (`KismetMathLibrary.MakeRotator` 0.0 0.0 _returnvalue_yaw)) AxisValue))

(event `InputAction|SwitchBow`
  (params (Key :type "Key Structure"))
  ;[0 0 0] Weapon Switching
  (:`Pressed`
    (if (`self.Has Weapon?` "NewEnumerator1")
      (bind _weapon_data (`self.Get Weapon From Data Table` "NewEnumerator1"))
      (`self.Equip Weapon` _weapon_data))))

(event `self.ReceiveTick`
  (params (DeltaSeconds :type "Float (single-precision)"))
  ;[0 0 0] Weapon Bob Animation
  (bind _asbp_player_weapon_base (cast `/Game/RetroFPS/Blueprints/Player/BP_PlayerWeaponBase` (`ChildActorComponent.ChildActor` (`self.Weapon`))))
  (`/Game/RetroFPS/Blueprints/Player/BP_PlayerWeaponBase.Weapon Bobbing` _asbp_player_weapon_base (> (`KismetMathLibrary.VSize` (`MovementComponent.Velocity` (`self.CharacterMovement`))) 0.0) DeltaSeconds))

(event `InputAction|SwitchAxe`
  (params (Key :type "Key Structure"))
  ;[0 0 0] Weapon Switching
  (:`Pressed`
    (if (`self.Has Weapon?` "NewEnumerator2")
      (bind _weapon_data (`self.Get Weapon From Data Table` "NewEnumerator2"))
      (`self.Equip Weapon` _weapon_data))))

(event `InputAxis|VerticalMovement`
  (params (AxisValue :type "Float (single-precision)"))
  (bind (_returnvalue_roll _returnvalue_pitch _returnvalue_yaw) (`KismetMathLibrary.BreakRotator` (`self.GetControlRotation`)))
  ;[0 0 0] Movement
  (`self.AddMovementInput` (`KismetMathLibrary.GetForwardVector` (`KismetMathLibrary.MakeRotator` 0.0 0.0 _returnvalue_yaw)) AxisValue))

(event `InputAxis|MouseLookHorizontal`
  (params (AxisValue :type "Float (single-precision)"))
  ;[0 0 0] Mouse Look
  (`self.AddControllerYawInput` AxisValue))

(event `Equip Weapon`
  (params (Weapon :type "/Game/RetroFPS/Blueprints/Strucs/ST_WeaponData Structure"))
  (bind _current_weapon_weaponname (break `/Game/RetroFPS/Blueprints/Strucs/ST_WeaponData` (`self.Current Weapon`)))
  (bind _current_weapon_weaponname_2 (break `/Game/RetroFPS/Blueprints/Strucs/ST_WeaponData` (`self.Current Weapon`)))
  ;[0 0 0] Equip Weapon
  (bind _output_get (set `self.Current Weapon` Weapon))
  (bind _weapon_actor (`self.Initialize Weapon` (`.Weapon_6_3ADB765C4CA328F569F1CEBCA6E50785` (break `/Game/RetroFPS/Blueprints/Strucs/ST_WeaponData` _output_get))))
  (bind _asbp_player_weapon_base (cast `/Game/RetroFPS/Blueprints/Player/BP_PlayerWeaponBase` _weapon_actor))
  (`MovieSceneSequencePlayer.Play` (`ActorSequenceComponent.SequencePlayer` (`/Game/RetroFPS/Blueprints/Player/BP_PlayerWeaponBase.Weapon Draw` _asbp_player_weapon_base)))
  (`/Game/RetroFPS/Blueprints/Widgets/WBP_HUD.Switch Weapon` (`self.HUD`) _current_weapon_weaponname_2)
  (`self.Update UI`)
  (switch `/Game/RetroFPS/Blueprints/ENUMs/ENUM_WeaponList` _current_weapon_weaponname
    (:`NewEnumerator0`
      (set `self.Weapon Fire Tag Container` (struct)))
    (:`NewEnumerator1`
      (set `self.Weapon Fire Tag Container` (struct :`GameplayTags` (struct :`(TagName` "Player.Weapon.Bow.Fire")))))
    (:`NewEnumerator2`
      (set `self.Weapon Fire Tag Container` (struct :`GameplayTags` (struct :`(TagName` "Player.Weapon.Axe.Attack")))))))

(event `InputAxis|MouseLookVertical`
  (params (AxisValue :type "Float (single-precision)"))
  ;[0 0 0] Mouse Look
  (`self.AddControllerPitchInput` AxisValue))

(event `Item Pickup`
  ;[0 0 0] Item Pickup
  (`self.Update UI`)
  (bind (_direction _alpha) (`Timeline|Pickup Flash` :!via `PlayFromStart`)
    (:`Update`
      (`/Game/RetroFPS/Blueprints/Widgets/WBP_HUD.Set Flash Color` (`self.HUD`) (struct :`R` 0.022484 :`G` 0.018397 :`B` 0.619792 :`A` 1.0) _alpha))))

(event `InputAction|FireWeapon`
  (params (Key :type "Key Structure"))
  ;[0 0 0] Fire Weapon
  (:`Pressed`
    (`AbilitySystemComponent.TryActivateAbilitiesByTag` (`self.AbilitySystemComponent`) (`self.Weapon Fire Tag Container`) false)))

(event `self.Take Damage`
  (params (`Cue Data` :type "GameplayCueParameters Structure"))
  ;[0 0 0] Take Damage
  (`parent.Take Damage` `Cue Data`)
  (`self.Update UI`)
  (bind (_direction _alpha) (`Timeline|Damage Flash` :!via `PlayFromStart`)
    (:`Update`
      (`/Game/RetroFPS/Blueprints/Widgets/WBP_HUD.Set Flash Color` (`self.HUD`) (struct :`R` 1.0 :`B` 0.032635 :`A` 1.0) _alpha))))

(event `Pickup Weapon`
  (params (Weapon :type "/Game/RetroFPS/Blueprints/ENUMs/ENUM_WeaponList Enum" :default "NewEnumerator0"))
  ;[0 0 0] Weapon Pickup
  (bind (_weapon_data _weapon_found) (`self.Get Weapon From Data Table` Weapon))
  (if _weapon_found
    (bind _output_get (set `self.Weapon To Pickup` _weapon_data))
    (if (not (`self.Has Weapon?` (`.WeaponName_13_59E2AB9E4679076EFA76ECAD738CC5DB` (break `/Game/RetroFPS/Blueprints/Strucs/ST_WeaponData` _output_get))))
      (`self.Add Weapon`))
    (else
      (`KismetSystemLibrary.PrintString` "Weapon does not exist in Data Table!"))))

(event `Add Weapon`
  (bind _weapon_to_pickup (`self.Weapon To Pickup`))
  ;[0 0 0] Add Weapon
  (`KismetArrayLibrary.Array_Add` (`self.Player Weapons`) _weapon_to_pickup)
  (`self.Equip Weapon` _weapon_to_pickup))

(fn `Get Weapon From Data Table`
  (params (Weapon :type "/Game/RetroFPS/Blueprints/ENUMs/ENUM_WeaponList Enum" :default "NewEnumerator0"))
  (returns (`Weapon Data` :type "/Game/RetroFPS/Blueprints/Strucs/ST_WeaponData Structure") (`Weapon Found` :type Boolean))
  (locals (`Weapon Exists` :type Boolean) (`Weapon To Equip` :type "/Game/RetroFPS/Blueprints/Strucs/ST_WeaponData Structure"))
  (bind _outrownames (`DataTableFunctionLibrary.GetDataTableRowNames` "/Game/RetroFPS/Blueprints/Weapons/DT_RetroFPSWeapons.DT_RetroFPSWeapons"))
  (for _array_element _outrownames
    (bind _returnvalue (`|GetDataTableRow` "/Game/RetroFPS/Blueprints/Weapons/DT_RetroFPSWeapons.DT_RetroFPSWeapons" _array_element)
      (:`then`
        (if (`|EnumEquality` Weapon (`.WeaponName_13_59E2AB9E4679076EFA76ECAD738CC5DB` (break `/Game/RetroFPS/Blueprints/Strucs/ST_WeaponData` _returnvalue)))
          (set `local.Weapon Exists` true)
          (set `local.Weapon To Equip` _returnvalue)
          (break)))))
  (return (`local.Weapon To Equip`) (`local.Weapon Exists`)))

(fn `Has Weapon?`
  (params (ST_WeaponData :type "/Game/RetroFPS/Blueprints/ENUMs/ENUM_WeaponList Enum" :default "NewEnumerator0"))
  (returns (`Has Weapon?` :type Boolean))
  (locals (`Has Weapon` :type Boolean))
  (for _array_element (`self.Player Weapons`)
    (if (`|EnumEquality` (`.WeaponName_13_59E2AB9E4679076EFA76ECAD738CC5DB` (break `/Game/RetroFPS/Blueprints/Strucs/ST_WeaponData` _array_element)) ST_WeaponData)
      (set `local.Has Weapon` true)
      (break)))
  (return (`local.Has Weapon`)))

(fn `Initialize Weapon`
  (params (`In Class` :type "/Game/RetroFPS/Blueprints/Player/BP_PlayerWeaponBase Class Reference"))
  (returns (`Weapon Actor` :type "Actor Object Reference"))
  (bind _weapon (`self.Weapon`))
  (bind _childactor (`ChildActorComponent.ChildActor` _weapon))
  (`ChildActorComponent.SetChildActorClass` _weapon `In Class`)
  (if (`KismetSystemLibrary.DoesImplementInterface` _childactor "/Game/RetroFPS/Blueprints/Interfaces/IPlayerWeapon.IPlayerWeapon_C")
    (message `/Game/RetroFPS/Blueprints/Interfaces/IPlayerWeapon.Initialize Weapon` _childactor))
  (return _childactor))

(fn `Update UI`
  (bind _abilitysystemcomponent (`self.AbilitySystemComponent`))
  (bind _hud (`self.HUD`))
  (`TextBlock.SetText` (`/Game/RetroFPS/Blueprints/Widgets/WBP_HUD.HealthValue` _hud) (`KismetTextLibrary.Conv_DoubleToText` (`.ReturnValue` (`AbilitySystemBlueprintLibrary.GetFloatAttributeFromAbilitySystemComponent` _abilitysystemcomponent (struct :`AttributeName` "Health" :`Attribute` "/Script/Test.RetroFPSAttributeSet:Health" :`AttributeOwner` "/Script/CoreUObject.Class'/Script/Test.RetroFPSAttributeSet'"))) "HalfToEven"))
  (`TextBlock.SetText` (`/Game/RetroFPS/Blueprints/Widgets/WBP_HUD.ArmorValue` _hud) (`KismetTextLibrary.Conv_DoubleToText` (`.ReturnValue` (`AbilitySystemBlueprintLibrary.GetFloatAttributeFromAbilitySystemComponent` _abilitysystemcomponent (struct :`AttributeName` "Armor" :`Attribute` "/Script/Test.RetroFPSAttributeSet:Armor" :`AttributeOwner` "/Script/CoreUObject.Class'/Script/Test.RetroFPSAttributeSet'"))) "HalfToEven")))

(fn `UserConstructionScript`)
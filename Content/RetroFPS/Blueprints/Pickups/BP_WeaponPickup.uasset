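; BP_WeaponPickup is a weapon pickup in a retro FPS that grants the player a bow or axe when walked over.
; On overlap with BP_FPSPlayer, it passes its WeaponToAcquire value to PickupWeapon and destroys itself.
; The construction script sets the Item flipbook from WeaponToAcquire, so each placed instance shows its matching sprite, or none for None.
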(event `self.ReceiveActorBeginOverlap`
  (params (OtherActor :type "Actor Object Reference"))
  (bind _asbp_fpsplayer (cast `/Game/RetroFPS/Blueprints/Player/BP_FPSPlayer` OtherActor))
  (`/Game/RetroFPS/Blueprints/Player/BP_FPSPlayer.Pickup Weapon` _asbp_fpsplayer (`self.Weapon to Acquire`))
  (`self.K2_DestroyActor`))

(fn `UserConstructionScript`
  (bind _item (`self.Item`))
  (switch `/Game/RetroFPS/Blueprints/ENUMs/ENUM_WeaponList` (`self.Weapon to Acquire`)
    (:`NewEnumerator0`
      (`PaperFlipbookComponent.SetFlipbook` _item null))
    (:`NewEnumerator1`
      (`PaperFlipbookComponent.SetFlipbook` _item "/Game/RetroFPS/Flipbooks/Pickups/FB_Bow_Pickup.FB_Bow_Pickup"))
    (:`NewEnumerator2`
      (`PaperFlipbookComponent.SetFlipbook` _item "/Game/RetroFPS/Flipbooks/Pickups/FB_Axe_Pickup.FB_Axe_Pickup"))))